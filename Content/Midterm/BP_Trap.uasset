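; BP_Trap is a trap actor that damages the first-person player on overlap with its Trap component.
; Overlap plays a timeline that drives the relative location of OPM0041 through a lerp, though both endpoints are zero.
; A DoOnce on the timeline update subtracts 50 health a single time.
; At zero health it shows WP_Dead, sets IsDead, destroys the player character and opens MainMenu after a delay.
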(event OnComponentBeginOverlap(trap)
  (params (OverlappedComponent :type Primitive%20Component%20Object%20Reference) (OtherActor :type Actor%20Object%20Reference) (OtherComp :type Primitive%20Component%20Object%20Reference) (OtherBodyIndex :type Integer) (bFromSweep :type Boolean) (SweepResult :type Hit%20Result%20Structure%20%28by%20ref%29))
  (bind _asbp_first_person_character (Utilities|Casting|CastToBP_FirstPersonCharacter OtherActor))
  (if true
    (bind _newtrack_0 (Timeline|Timeline Play)
      (:Update
        (Transformation|SetRelativeLocation (Variables|Default|GetOPM0041) (Math|Vector|Lerp(Vector) "0, 0, 0" "0, 0, 0" _newtrack_0) false false)
        (Utilities|FlowControl|DoOnce false
          (:Completed
            (bind _output_get (Variables|/Game/FirstPerson/Blueprints/BP_FirstPersonCharacter.BP_FirstPersonCharacter_C|Sethealth _asbp_first_person_character (- (Variables|/Game/FirstPerson/Blueprints/BP_FirstPersonCharacter.BP_FirstPersonCharacter_C|Gethealth _asbp_first_person_character) 5e+01)))
            (if (<= _output_get 0.0)
              (bind _returnvalue (UserInterface|CreateWidget "/Game/Midterm/WP_Dead.WP_Dead_C" (Game|GetPlayerController 0)))
              (UserInterface|Viewport|AddtoViewport _returnvalue 0)
              (Variables|/Game/FirstPerson/Blueprints/BP_FirstPersonCharacter.BP_FirstPersonCharacter_C|SetIsDead _asbp_first_person_character true)
              (Actor|DestroyActor (Game|GetPlayerCharacter 0))
              (Utilities|FlowControl|Delay 2.0)
              (Game|OpenLevel(byName) "MainMenu"))))))))

(event EventBeginPlay)

(event Collision|EventActorBeginOverlap
  (params (OtherActor :type Actor%20Object%20Reference)))

(event EventTick
  (params (DeltaSeconds :type Float%20%28single-precision%29)))

(fn ConstructionScript)