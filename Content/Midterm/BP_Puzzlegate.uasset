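; BP_Puzzlegate is a puzzle gate that swings open once enough collectible items have been gathered.
; CollectItem increments a counter, and OpenDoorCheck compares it to the maximum, firing OpenDoor only once through a DoOnce.
; OpenDoor plays a timeline that lerps the door's relative yaw from closed to open.
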(event Custom|Open%20Door
  (bind _door_rotation (Timeline|Timeline Play)
    (:Update
      (Transformation|SetRelativeRotation (Variables|Default|GetDoor) (Math|Rotator|MakeRotator 0.0 0.0 (Math|Float|Lerp 0.0 1.2e+02 _door_rotation)) false false))))

(event Custom|Collect%20Item
  (Math|Integer|IncrementInt (Variables|Default|GetCurrentItemsCollected)))

(event Custom|Open%20Door%20Check
  (if (>= (Variables|Default|GetCurrentItemsCollected) (Variables|Default|GetMAXItemsCollactable))
    (Utilities|FlowControl|DoOnce false
      (:Completed
        (CallFunction|OpenDoor)))))

(event Collision|EventActorBeginOverlap
  (params (OtherActor :type Actor%20Object%20Reference)))

(event EventTick
  (params (DeltaSeconds :type Float%20%28single-precision%29)))

(fn ConstructionScript)