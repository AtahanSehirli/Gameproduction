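; BP_Lava is a hazard actor that damages the first-person player character while they stand in it.
; A box overlap casts to BP_FirstPersonCharacter, stores it, and calls TakeDamage, repeating after a short delay while the overlap continues.
; The delayed return to MainMenu sits behind a constant-false branch, so it never runs, and leftover death-handling nodes are disconnected.
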(event OnComponentBeginOverlap(Box)
  (params (OverlappedComponent :type Primitive%20Component%20Object%20Reference) (OtherActor :type Actor%20Object%20Reference) (OtherComp :type Primitive%20Component%20Object%20Reference) (OtherBodyIndex :type Integer) (bFromSweep :type Boolean) (SweepResult :type Hit%20Result%20Structure%20%28by%20ref%29))
  (bind _asbp_first_person_character (Utilities|Casting|CastToBP_FirstPersonCharacter OtherActor))
  (bind _output_get (Variables|Default|SetPlayer%20Character _asbp_first_person_character))
  (Default|TakeDamage _output_get :!label _label)
  (if false
    (Utilities|FlowControl|Delay 2.0)
    (Game|OpenLevel(byName) "MainMenu")
    (else
      (Utilities|FlowControl|Delay 0.5)
      (if (Collision|IsOverlappingActor (Variables|Default|GetPlayer%20Character) :!class /Script/Engine.Actor)
        (goto _label)))))

(event EventBeginPlay)

(event Collision|EventActorBeginOverlap
  (params (OtherActor :type Actor%20Object%20Reference)))

(event EventTick
  (params (DeltaSeconds :type Float%20%28single-precision%29)))

(fn ConstructionScript)