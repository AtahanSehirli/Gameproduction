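; BP_KeyButton is a single clickable key for a keypad, labeled through a text component set from NoText in the construction script.
; Clicking sends its value plus confirm and backspace flags to the referenced keypad actor's ButtonEntered.
; Cursor hover changes the button's material by clearing the slot override, while leaving or calling ResetButton restores M_Solid.
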(event OnBeginCursorOver(Button)
  (params (TouchedComponent :type Primitive%20Component%20Object%20Reference))
  (Rendering|Material|SetMaterial (Variables|Default|GetButton) 0 0))

(event OnEndCursorOver(Button)
  (params (TouchedComponent :type Primitive%20Component%20Object%20Reference))
  (Rendering|Material|SetMaterial (Variables|Default|GetButton) 0 "/Game/LevelPrototyping/Materials/M_Solid.M_Solid"))

(event OnClicked(Button)
  (params (TouchedComponent :type Primitive%20Component%20Object%20Reference) (ButtonPressed :type Key%20Structure :default "None"))
  (CallFunction|ButtonEntered (.KeyPadActorRef (Variables|Default|GetKeyPadActorRef)) (Variables|Default|GetNoText) (Variables|Default|GetConfrimButton) (Variables|Default|GetBackspacebutton)))

(event Custom|ResetButton
  (Rendering|Material|SetMaterial (Variables|Default|GetButton) 0 "/Game/LevelPrototyping/Materials/M_Solid.M_Solid"))

(event EventBeginPlay)

(event Collision|EventActorBeginOverlap
  (params (OtherActor :type Actor%20Object%20Reference)))

(event EventTick
  (params (DeltaSeconds :type Float%20%28single-precision%29)))

(fn ConstructionScript
  (Rendering|Components|TextRender|SetText (Variables|Default|GetButtonNo) (Variables|Default|GetNoText)))